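; Clicker tower actor built from stacked, randomly colored cylinder meshes, generated in the construction script.
; OnHit destroys the hit segment, lowers the tower by one segment height, updates BPBorder's rotation rate and refreshes the HUD score.
; While CanSpawn is true, each hit also adds a segment on top and increments Score.
; Every tenth point spawns a randomly true-or-false BP_Bonus, removed by timer after a few seconds.
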(event EventBeginPlay
  (bind _asbp_hud (Utilities|Casting|CastToBP_HUD (HUD|GetHUD (Game|GetPlayerController 0))))
  (Variables|Default|SetAs%20BP%20HUD _asbp_hud))

(event Collision|EventActorBeginOverlap
  (params (OtherActor :type Actor%20Object%20Reference)))

(event EventTick
  (params (DeltaSeconds :type Float%20%28single-precision%29)))

(event EventOnHit
  (params (HitComponent :type Primitive%20Component%20Object%20Reference))
  (Components|DestroyComponent HitComponent)
  (Utilities|FlowControl|Sequence
    (:then_0
      (if (Variables|Default|GetCanSpawn)
        (CallFunction|MountSylinder 1)
        (Math|Integer|IncrementInt (Variables|Default|GetScore)
          (:%20%20
            (CallFunction|TrySpawnBonus)))))
    (:then_1
      (Transformation|AddActorLocalOffset (Math|Vector|MakeVector 0.0 0.0 (Variables|Default|GetOffset)) false false)
      (Default|UpdateRotationRate (Variables|Default|GetBP_Border) 1.0)
      (Default|UpdateScore (Variables|/Game/Clicker/Blueprints/BP_HUD.BP_HUD_C|GetUI (Variables|Default|GetAs%20BP%20HUD)) (Variables|Default|GetScore)))))

(fn ConstructionScript
  (CallFunction|MountSylinder (Variables|Default|GetNumOfSylinders)))

(fn MountSylinder
  (params (NumOfCylinders :type Integer))
  (LocalVariables|SetLocalNumOfCylinders NumOfCylinders)
  (if (> (LocalVariables|GetLocalNumOfCylinders) 0)
    (for _index (range 0 (- (LocalVariables|GetLocalNumOfCylinders) 1))
      (bind _returnvalue (AddComponent|AddStaticMeshComponent false (Variables|Default|GetLastTransform)))
      (LocalVariables|SetLocalMeshComponent _returnvalue)
      (bind _returnvalue_2 (Rendering|Material|CreateDynamicMaterialInstance (LocalVariables|GetLocalMeshComponent) 0 (Rendering|Material|GetMaterial (LocalVariables|GetLocalMeshComponent) 0) "None" :!class /Script/Engine.PrimitiveComponent))
      (Rendering|Material|SetVectorParameterValue _returnvalue_2 "Color" (Utilities|Struct|MakeLinearColor (Math|Random|RandomFloatinRange 0.0 1.0) (Math|Random|RandomFloatinRange 0.0 1.0) (Math|Random|RandomFloatinRange 0.0 1.0) 0.0) :!class /Script/Engine.MaterialInstanceDynamic)
      (Variables|Default|SetLastTransform (Math|Transform|MakeTransform (Math|Vector|MakeVector (.x (.location (Variables|Default|GetLastTransform))) (.y (.location (Variables|Default|GetLastTransform))) (+ (.z (.location (Variables|Default|GetLastTransform))) (.z (- (.Max (Components|StaticMesh|GetLocalBounds (LocalVariables|GetLocalMeshComponent))) (.Min (Components|StaticMesh|GetLocalBounds (LocalVariables|GetLocalMeshComponent))))))) (.rotation (Variables|Default|GetLastTransform)) (.scale (Variables|Default|GetLastTransform)))))
    (Variables|Default|SetOffset (.z (- (.Min (Components|StaticMesh|GetLocalBounds (LocalVariables|GetLocalMeshComponent))) (.Max (Components|StaticMesh|GetLocalBounds (LocalVariables|GetLocalMeshComponent))))))))

(fn TrySpawnBonus
  (if (== (Math|Integer|%(Integer) (Variables|Default|GetScore) 10) 0)
    (bind _returnvalue (Game|SpawnActorfromClass "/Game/Clicker/Blueprints/BP_Bonus.BP_Bonus_C" (Transformation|GetActorTransform (Variables|Default|GetBonusePoint)) "Undefined" "MultiplyWithRoot" 0 (Math|Random|RandomBool) (Variables|Default|GetBP_Border) 0))
    (Variables|Default|SetBP_Bonus _returnvalue)
    (Utilities|Time|SetTimerbyFunctionName 0 "DestroyBonus" 5.0)))

(fn DestroyBonus
  (bind _bp_bonus (Variables|Default|GetBP_Bonus)
    (:then
      (Actor|DestroyActor _bp_bonus)
      (Variables|Default|SetBP_Bonus 0))
    (:else)))