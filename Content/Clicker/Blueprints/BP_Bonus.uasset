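; BP_Bonus is a hittable bonus actor for the Clicker game with a good or bad variant set by IsTrueBonuse.
; When hit, it passes a negative rotation rate change to BPBorder for a true bonus or a positive one otherwise, then destroys itself.
; The construction script sets the static mesh from that flag.
; An unconnected green/red dynamic material tint remains in the construction script but never runs.
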(event EventBeginPlay)

(event Collision|EventActorBeginOverlap
  (params (OtherActor :type Actor%20Object%20Reference)))

(event EventTick
  (params (DeltaSeconds :type Float%20%28single-precision%29)))

(event EventOnHit
  (params (HitComponent :type Primitive%20Component%20Object%20Reference))
  (Default|UpdateRotationRate (Variables|Default|GetBP_Border) (Math|Float|SelectFloat -1e+01 1e+01 (Variables|Default|GetIsTrueBonuse)))
  (Actor|DestroyActor))

(fn ConstructionScript
  (Components|StaticMesh|SetStaticMesh (Variables|Default|GetStaticMesh) (select (Variables|Default|GetIsTrueBonuse) "/Game/Clicker/Meshes/CristalBonuse/Green/scene.scene" "/Game/Clicker/Meshes/CristalBonuse/Red/scene.scene")))