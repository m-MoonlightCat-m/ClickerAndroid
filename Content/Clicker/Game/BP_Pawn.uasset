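; Player pawn for the Clicker game that spawns a BP_Projectile at its Scene component's transform on an upward touch swipe.
; Touch press records the start point, and Tick watches for any finger movement while held.
; The first movement passes a DoOnce, re-armed on release, and its dominant axis sets the direction, so firing happens mid-touch.
; Horizontal and downward swipes trigger nothing.
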(event Custom|Fire
  (Game|SpawnActorfromClass "/Game/Clicker/Blueprints/BP_Projectile.BP_Projectile_C" (Transformation|GetWorldTransform (Variables|Default|GetScene)) "Undefined" "MultiplyWithRoot" 0 0))

(event EventBeginPlay)

(event Collision|EventActorBeginOverlap
  (params (OtherActor :type Actor%20Object%20Reference)))

(event EventTick
  (params (DeltaSeconds :type Float%20%28single-precision%29))
  (bind _returnvalue (Game|GetPlayerController 0))
  (bind (_locationx _locationy) (Class|PlayerController|GetInputTouchState _returnvalue "Touch1"))
  (bind _returnvalue_2 (Math|Vector2D|MakeVector2D _locationx _locationy))
  (if (Variables|Default|GetIsTouch)
    (if (> (Math|Vector2D|Vector2DLength (- (Variables|Default|GetTouchStart2DVector) _returnvalue_2)) 0.0)
      (Utilities|FlowControl|DoOnce false
        (:Completed
          (Variables|Default|SetTouchEnd2DVector _returnvalue_2)
          (if (> (Math|Float|Absolute(Float) (.X (Math|Vector2D|BreakVector2D (- (Variables|Default|GetTouchStart2DVector) (Variables|Default|GetTouchEnd2DVector))))) (Math|Float|Absolute(Float) (.Y (Math|Vector2D|BreakVector2D (- (Variables|Default|GetTouchStart2DVector) (Variables|Default|GetTouchEnd2DVector))))))
            (if (> (.X (Math|Vector2D|BreakVector2D (- (Variables|Default|GetTouchStart2DVector) (Variables|Default|GetTouchEnd2DVector)))) 0.0)
              _)
            (elif (not (> 0.0 (.Y (Math|Vector2D|BreakVector2D (- (Variables|Default|GetTouchStart2DVector) (Variables|Default|GetTouchEnd2DVector))))))
              (CallFunction|Fire))))))))

(event Input|TouchEvents|InputTouch
  (params (Location :type Vector) (FingerIndex :type ETouchIndex%20Enum))
  (bind _returnvalue (Game|GetPlayerController 0))
  (bind (_locationx _locationy) (Class|PlayerController|GetInputTouchState _returnvalue "Touch1"))
  (bind _returnvalue_2 (Math|Vector2D|MakeVector2D _locationx _locationy))
  (:Pressed
    (Variables|Default|SetIsTouch true)
    (Variables|Default|SetTouchStart2DVector _returnvalue_2))
  (:Released
    (Variables|Default|SetIsTouch false)
    (Utilities|FlowControl|DoOnce false) ; enters at Reset
  ))

(fn ConstructionScript)